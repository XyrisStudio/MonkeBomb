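; Volume actor that supplies occlusion settings to Ultra Dynamic Sky and Ultra Dynamic Weather, with separate values for each.
; The construction script adds a box, sphere or capsule collision component sized from its properties.
; When set to block weather particles, it queries the first weather interface actor for the particle collision channel and blocks it.
; GetOcclusionResult returns the weather or sky occlusion setting as requested.
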(fn ConstructionScript
  (switch Utilities|FlowControl|Switch|SwitchonUDS_OcclusionShape (Variables|Shape|GetCollision%20Shape)
    (:NewEnumerator0
      (bind _returnvalue (AddComponent|AddBoxComponent false))
      (Variables|Default|SetCollision%20Component _returnvalue)
      (Components|Box|SetBoxExtent _returnvalue (Variables|Shape|GetBox%20Extent) true))
    (:NewEnumerator1
      (bind _returnvalue_2 (AddComponent|AddSphereComponent false))
      (Variables|Default|SetCollision%20Component _returnvalue_2)
      (Components|Sphere|SetSphereRadius _returnvalue_2 (Variables|Shape|GetSphere%20Radius) true))
    (:NewEnumerator2
      (bind _returnvalue_3 (AddComponent|AddCapsuleComponent false))
      (Variables|Default|SetCollision%20Component _returnvalue_3)
      (Components|Capsule|SetCapsuleRadius _returnvalue_3 (Variables|Shape|GetSphere%20Radius) true)
      (Components|Capsule|SetCapsuleHalfHeight _returnvalue_3 (Variables|Shape|GetCapsule%20Half%20Height) true)))
  (if (Variables|Occlusion|GetBlock%20Weather%20Particles)
    (bind _outactors (Actor|GetAllActorswithInterface "/Game/Resources/_External/Sky/Blueprints/Weather_Effects/System/Ultra_Dynamic_Weather_Interface.Ultra_Dynamic_Weather_Interface_C"))
    (if (Utilities|Array|IsValidIndex _outactors)
      (bind _channel (Class|UltraDynamicWeatherInterface|GetWeatherParticleCollisionChannel(Message) (Utilities|Array|Get(acopy) _outactors)))
      (Collision|SetCollisionResponsetoChannel (Variables|Default|GetCollision%20Component) _channel "ECR_Block"))))

(fn GetOcclusionResult
  (params (Weather :type Boolean))
  (return (select Weather (Variables|Occlusion|GetAffect%20Occlusion%20on%20Ultra%20Dynamic%20Weather) (Variables|Occlusion|GetAffect%20Occlusion%20on%20Ultra%20Dynamic%20Sky))))
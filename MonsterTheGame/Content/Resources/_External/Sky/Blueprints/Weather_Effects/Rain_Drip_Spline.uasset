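; Spline actor for Ultra Dynamic Weather that spawns rain drips and splashes along an editable path.
; Creates one Niagara emitter per spline segment, passing Bezier points, length share and downward-extended fixed bounds.
; On tick, unless weather is ignored, Wet, Raining and Wind Force from the parameter collection update spawn rate, splashes and curl noise.
; The weather actor supplies collision channel, lighting settings and mobile material choice.
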(event EventResetEmitters
  (Utilities|FlowControl|Delay 0.05)
  (CallFunction|UpdatewithWeather)
  (Niagara|ReinitializeSystem (Variables|Default|GetDrip%20Emitters)))

(event EventForceStartup
  (Variables|Default|SetRuntime true)
  (CallFunction|CreateCurveData)
  (CallFunction|UpdateStaticNiagaraParameters)
  (CallFunction|UpdatewithWeather)
  (if (not (Variables|Default|GetIgnore%20Weather%20State))
    (Utilities|FlowControl|Delay (Math|Random|RandomFloatinRange 0.0 3.0))
    (Actor|Tick|SetActorTickEnabled true)))

(event EventEditorUpdate
  (CallFunction|UpdatewithWeather))

(event EventTick
  (params (DeltaSeconds :type Float%20%28single-precision%29))
  (CallFunction|UpdatewithWeather))

(event EventBeginPlay
  (bind _returnvalue (Actor|GetActorOfClass "/Game/Resources/_External/Sky/Blueprints/Ultra_Dynamic_Weather.Ultra_Dynamic_Weather_C"))
  (if (Variables|/Game/Resources/_External/Sky/Blueprints/Ultra_Dynamic_Weather.Ultra_Dynamic_Weather_C|GetInitialized _returnvalue)
    (Variables|Default|SetRuntime true)
    (CallFunction|CreateCurveData)
    (CallFunction|UpdateStaticNiagaraParameters)
    (CallFunction|UpdatewithWeather)
    (if (not (Variables|Default|GetIgnore%20Weather%20State))
      (Utilities|FlowControl|Delay (Math|Random|RandomFloatinRange 0.0 3.0))
      (Actor|Tick|SetActorTickEnabled true))))

(fn ConstructionScript
  (Variables|Default|SetRefresh false)
  (CallFunction|CreateCurveData)
  (CallFunction|UpdateStaticNiagaraParameters)
  (CallFunction|UpdatewithWeather))

(fn UpdatewithWeather
  (bind _returnvalue (Rendering|Material|GetScalarParameterValue "/Game/Resources/_External/Sky/Materials/Weather/UltraDynamicWeather_Parameters.UltraDynamicWeather_Parameters" "Wet" :!class /Script/Engine.KismetMaterialLibrary))
  (bind _returnvalue_2 (Rendering|Material|GetScalarParameterValue "/Game/Resources/_External/Sky/Materials/Weather/UltraDynamicWeather_Parameters.UltraDynamicWeather_Parameters" "Raining" :!class /Script/Engine.KismetMaterialLibrary))
  (LocalVariables|SetRaining (Math|Float|SelectFloat 1.0 _returnvalue_2 (Variables|Default|GetIgnore%20Weather%20State)))
  (Variables|Default|SetCurrent%20Spawn%20Rate (* (Math|Float|SelectFloat 1.0 (Math|Float|Clamp(Float) (+ _returnvalue_2 (* _returnvalue 0.01))) (Variables|Default|GetIgnore%20Weather%20State)) (+ (* (Variables|Default|GetSpawn%20Rate%20Per%20Meter) (/ (Spline|GetSplineLength (Variables|Default|GetSpline)) 1e+02)) (Variables|Default|GetExtra%20Spawn%20Rate))))
  (Effects|Components|ParticleSystem|SetFloatParameter (Variables|Default|GetDrip%20Emitters) "Spawn Rate" (Variables|Default|GetCurrent%20Spawn%20Rate))
  (Utilities|FlowControl|Sequence
    (:then_0
      (bind _output_get (Variables|Default|SetSystem%20Active (> (Variables|Default|GetCurrent%20Spawn%20Rate) 0.0)))
      (Components|Activation|SetActive (Variables|Default|GetDrip%20Emitters) _output_get false))
    (:then_1
      (if (Variables|Default|GetSystem%20Active)
        (bind _returnvalue_3 (Rendering|Material|GetVectorParameterValue "/Game/Resources/_External/Sky/Materials/Weather/UltraDynamicWeather_Parameters.UltraDynamicWeather_Parameters" "Wind Force" :!class /Script/Engine.KismetMaterialLibrary))
        (Effects|Components|ParticleSystem|SetFloatParameter (Variables|Default|GetDrip%20Emitters) "Curl Noise Force" (* (Math|Float|MapRangeClamped (Math|Vector|VectorLength (Math|Conversions|ToVector(LinearColor) _returnvalue_3)) 0.0 2e+03 42.0 1.4e+02) (Variables|Default|GetCurl%20Noise%20Force)))
        (Effects|Components|ParticleSystem|SetIntParameter (Variables|Default|GetDrip%20Emitters) "Splash Duplicate Count" (Math|Float|Round (Math|Float|MapRangeClamped (LocalVariables|GetRaining) 0.1 1.0 1.0 2.0)))
        (Effects|Components|ParticleSystem|SetFloatParameter (Variables|Default|GetDrip%20Emitters) "Splash Duplicate Range" (Math|Float|MapRangeClamped (LocalVariables|GetRaining) 0.0 1.0 0.0 6.0))))))

(fn CreateCurveData
  (bind _drip_emitters (Variables|Default|GetDrip%20Emitters))
  (bind _spline (Variables|Default|GetSpline))
  (bind _spline_2 (Variables|Default|GetSpline))
  (Spline|SetClosedLoop (Variables|Default|GetSpline) (Variables|Default|GetClosed%20Spline%20Loop) true)
  (Components|DestroyComponent _drip_emitters)
  (Utilities|Array|Clear _drip_emitters)
  (LocalVariables|SetNumber%20of%20Segments (Class|SplineComponent|GetNumberOfSplineSegments (Variables|Default|GetSpline)))
  (for _index (range 0 (- (LocalVariables|GetNumber%20of%20Segments) 1))
    (LocalVariables|SetSegment%20Index _index)
    (bind _returnvalue (AddComponent|AddNiagaraComponent false (Math|Transform|MakeTransform "0, 0, 0")))
    (bind _output_get (LocalVariables|SetCurrent%20Emitter _returnvalue))
    (Utilities|Array|Add (Variables|Default|GetDrip%20Emitters) _output_get)
    (Effects|Components|ParticleSystem|SetVectorParameter (LocalVariables|GetCurrent%20Emitter) "Curve Position A" (Spline|GetLocationatSplinePoint (Variables|Default|GetSpline) (LocalVariables|GetSegment%20Index) "Local"))
    (Effects|Components|ParticleSystem|SetVectorParameter (LocalVariables|GetCurrent%20Emitter) "Curve Handle A" (+ (Spline|GetLocationatSplinePoint (Variables|Default|GetSpline) (LocalVariables|GetSegment%20Index) "Local") (/ (Spline|GetLeaveTangentatSplinePoint (Variables|Default|GetSpline) (LocalVariables|GetSegment%20Index) "Local") 3.0)))
    (Effects|Components|ParticleSystem|SetVectorParameter (LocalVariables|GetCurrent%20Emitter) "Curve Position B" (Spline|GetLocationatSplinePoint (Variables|Default|GetSpline) (+ (LocalVariables|GetSegment%20Index) 1) "Local"))
    (Effects|Components|ParticleSystem|SetVectorParameter (LocalVariables|GetCurrent%20Emitter) "Curve Handle B" (+ (Spline|GetLocationatSplinePoint (Variables|Default|GetSpline) (+ (LocalVariables|GetSegment%20Index) 1) "Local") (* (/ (Spline|GetArriveTangentatSplinePoint (Variables|Default|GetSpline) (+ (LocalVariables|GetSegment%20Index) 1) "Local") 3.0) -1.0)))
    (Effects|Components|ParticleSystem|SetFloatParameter (LocalVariables|GetCurrent%20Emitter) "Spawn Distance Scale" (/ (- (Spline|GetDistanceAlongSplineatSplinePoint _spline_2 (+ (LocalVariables|GetSegment%20Index) 1)) (Spline|GetDistanceAlongSplineatSplinePoint _spline_2 (LocalVariables|GetSegment%20Index))) (Spline|GetSplineLength _spline_2)))
    (Effects|Components|ParticleSystem|SetIntParameter (LocalVariables|GetCurrent%20Emitter) "Collision Point Count" (Math|Float|Ceil (Math|Float|Clamp(Float) (- (Spline|GetDistanceAlongSplineatSplinePoint _spline_2 (+ (LocalVariables|GetSegment%20Index) 1)) (Spline|GetDistanceAlongSplineatSplinePoint _spline_2 (LocalVariables|GetSegment%20Index))) 1e+01 1e+03)))
    (LocalVariables|SetSegment%20Bounds%20Min "0, 0, 0")
    (LocalVariables|SetSegment%20Bounds%20Max "0, 0, 0")
    (for _index_2 (range 0 4)
      (LocalVariables|SetSegment%20Bounds%20Min (Math|Vector|VectorComponentMin (Spline|GetLocationatDistanceAlongSpline (Variables|Default|GetSpline) (Math|Float|Lerp (Spline|GetDistanceAlongSplineatSplinePoint _spline (LocalVariables|GetSegment%20Index)) (Spline|GetDistanceAlongSplineatSplinePoint _spline (+ (LocalVariables|GetSegment%20Index) 1)) (/ (Math|Conversions|ToFloat(Integer) _index_2) 4.0)) "Local") (LocalVariables|GetSegment%20Bounds%20Min)))
      (LocalVariables|SetSegment%20Bounds%20Max (Math|Vector|VectorComponentMax (Spline|GetLocationatDistanceAlongSpline (Variables|Default|GetSpline) (Math|Float|Lerp (Spline|GetDistanceAlongSplineatSplinePoint _spline (LocalVariables|GetSegment%20Index)) (Spline|GetDistanceAlongSplineatSplinePoint _spline (+ (LocalVariables|GetSegment%20Index) 1)) (/ (Math|Conversions|ToFloat(Integer) _index_2) 4.0)) "Local") (LocalVariables|GetSegment%20Bounds%20Max))))
    (LocalVariables|SetSegment%20Bounds%20Min (- (LocalVariables|GetSegment%20Bounds%20Min) "0,0,5000.000000"))
    (Class|NiagaraComponent|SetSystemFixedBounds (LocalVariables|GetCurrent%20Emitter) (Math|Box|MakeBox (LocalVariables|GetSegment%20Bounds%20Min) (LocalVariables|GetSegment%20Bounds%20Max))))
  (bind _returnvalue_2 (Actor|GetActorOfClass "/Game/Resources/_External/Sky/Blueprints/Ultra_Dynamic_Weather.Ultra_Dynamic_Weather_C"))
  (Class|NiagaraComponent|SetVariableMaterial (Variables|Default|GetDrip%20Emitters) "Splash Material" (select (Variables|/Game/Resources/_External/Sky/Blueprints/Ultra_Dynamic_Weather.Ultra_Dynamic_Weather_C|GetMobile _returnvalue_2) "/Game/Resources/_External/Sky/Materials/Weather/Splash_ParticleMat_Mobile.Splash_ParticleMat_Mobile" "/Game/Resources/_External/Sky/Materials/Weather/Splash_ParticleMat.Splash_ParticleMat")))

(fn UpdateStaticNiagaraParameters
  (Effects|Components|ParticleSystem|SetFloatParameter (Variables|Default|GetDrip%20Emitters) "Splash Percentage" (Variables|Default|GetSplash%20Frequency))
  (Effects|Components|ParticleSystem|SetFloatParameter (Variables|Default|GetDrip%20Emitters) "Drop Scale" (Variables|Default|GetDrops%20Scale))
  (Effects|Components|ParticleSystem|SetFloatParameter (Variables|Default|GetDrip%20Emitters) "Collision Head Start" (Variables|Default|GetCollision%20Line%20Trace%20Head%20Start))
  (bind _returnvalue (Actor|GetActorOfClass "/Game/Resources/_External/Sky/Blueprints/Ultra_Dynamic_Weather.Ultra_Dynamic_Weather_C"))
  (bind _channel (Default|GetWeatherParticleCollisionChannel _returnvalue))
  (Effects|Components|ParticleSystem|SetIntParameter (Variables|Default|GetDrip%20Emitters) "Particle Collision Channel" (Math|Conversions|ToInteger(Byte) _channel))
  (Effects|Components|ParticleSystem|SetFloatParameter (Variables|Default|GetDrip%20Emitters) "Ambient Intensity" (Variables|/Game/Resources/_External/Sky/Blueprints/Ultra_Dynamic_Weather.Ultra_Dynamic_Weather_C|GetRain%20Ambient%20Light%20Intensity _returnvalue))
  (Effects|Components|ParticleSystem|SetFloatParameter (Variables|Default|GetDrip%20Emitters) "Refraction Intensity" (Variables|/Game/Resources/_External/Sky/Blueprints/Ultra_Dynamic_Weather.Ultra_Dynamic_Weather_C|GetRain%20Refraction%20Intensity _returnvalue)))